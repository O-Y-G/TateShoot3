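; Spline-following enemy base Blueprint for TateShoot, derived from a parent enemy class.
; On BeginPlay it runs the parent logic, then plays a timeline from the start.
; The timeline's Alpha, scaled by spline length, gives the distance along the spline at which the Sphere component is placed in world space.
; Overlap and Tick events are disabled placeholders, and the construction script only calls the parent.
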(event `self.ReceiveBeginPlay`
  (bind _spline (`self.Spline`))
  (`parent.ReceiveBeginPlay`)
  (bind (_direction _alpha) (`Timeline|Timeline_Spline` :!via `PlayFromStart`)
    (:`Update`
      (`SceneComponent.K2_SetWorldTransform` (`self.Sphere`) (`KismetMathLibrary.MakeTransform` (`SplineComponent.GetLocationAtDistanceAlongSpline` _spline (* (`SplineComponent.GetSplineLength` _spline) _alpha) "World")) false false))))

(fn `UserConstructionScript`
  (`parent.UserConstructionScript`))